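; BP_Pixel is a short-lived actor that colors itself by its distance from the first-person character's camera.
; On BeginPlay it creates a dynamic emissive material, caches its location and destroys itself after LifeTime.
; A looping timer with a randomized start repeatedly samples a color curve using that distance.
; SetColorOnRed, noted for NPC collisions, pauses the timer and turns the pixel red.
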(event `self.ReceiveBeginPlay`
  ; Create dynamic material
  (bind _returnvalue (`KismetMaterialLibrary.CreateDynamicMaterialInstance` "/Game/Project/MaterialLibrary/Materials/PixelMaterials/M_PixellBasicMaterial.M_PixellBasicMaterial"))
  (set `self.DynamicMaterial` _returnvalue)
  (`PrimitiveComponent.SetMaterial` (`self.Pixel`) 0 (`self.DynamicMaterial`))
  ; Get actor locaition
  (set `self.PixelLocaition` (`self.K2_GetActorLocation`))
  ; Change color
  (`self.ChangeColor`)
  (bind _returnvalue_2 (`KismetSystemLibrary.K2_SetTimerDelegate` (delegate `ChangeColor`) 0.4 true true 0.0 0.2))
  (set `self.Timer` _returnvalue_2)
  ; Destroy object
  (`KismetSystemLibrary.Delay` (`self.LifeTime`))
  (`self.K2_DestroyActor`))

(event `ChangeColor`
  ; Set material
  (`MaterialInstanceDynamic.SetVectorParameterValue` (`self.DynamicMaterial`) "Emissive Color" (`CurveLinearColor.GetLinearColorValue` (`self.CurveColor`) (`KismetMathLibrary.Vector_Distance` (`/Game/FirstPerson/Blueprints/BP_FirstPersonCharacter.CameraLocaition` (`self.As BP First Person Character`)) (`self.PixelLocaition`)))))

(event `SetColorOnRed`
  ; Set material if pixel colaps with NPC
  (`KismetSystemLibrary.K2_PauseTimerHandle` (`self.Timer`))
  (`MaterialInstanceDynamic.SetVectorParameterValue` (`self.DynamicMaterial`) "Emissive Color" (struct :`R` 1.0 :`A` 1.0)))

(fn `UserConstructionScript`)