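; Lidar scanner component for the first-person character that paints surfaces with spawned BP_Pixel dots while the IA_LidarActivate input is held.
; A fast looping timer fires randomly spread Visibility traces from the camera, with the mouse wheel adjusting spread within limits.
; Each hit spawns a collision-free pixel unless its physical material is PM_NotRecetiveToLidar.
; A placeholder check colors pixels red when the hit actor matches BP_NPC.
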(event `self.ReceiveBeginPlay`
  ; Cast to FirstPersonCharacter
  (bind _asbp_first_person_character (cast `/Game/FirstPerson/Blueprints/BP_FirstPersonCharacter` (`GameplayStatics.GetPlayerPawn` 0)))
  (bind _output_get (set `self.As BP First Person Character` _asbp_first_person_character))
  ; Get First Person Camera
  (set `self.First Person Camera` (`/Game/FirstPerson/Blueprints/BP_FirstPersonCharacter.FirstPersonCamera` _output_get))
  ; Timer
  (`KismetSystemLibrary.K2_SetTimerDelegate` (delegate `SetTimer`) 0.001 true))

(event `SetTimer`
  ; Timer
  (`self.TimerResult`))

(event `TimerResult`
  ; Lidar line trace
  (if (`self.inLidarMode`)
    (`self.Lidar`)))

(event `EnhancedInput|/Game/Input/Actions/IA_LidarActivate`
  (params (ActionValue :type Boolean) (ElapsedSeconds :type "Float (double-precision)") (TriggeredSeconds :type "Float (double-precision)") (InputAction :type "InputAction Object Reference" :default "/Game/Input/Actions/IA_LidarActivate.IA_LidarActivate"))
  ; Set var inLidarMode
  (:`Triggered`
    (set `self.inLidarMode` true))
  (:`Completed`
    (set `self.inLidarMode` false)))

(event `Lidar`
  (bind _rangeinrandom (`self.RangeInRandom`))
  (bind (_returnvalue_location _returnvalue_rotation) (`KismetMathLibrary.BreakTransform` (`SceneComponent.K2_GetComponentToWorld` (`self.First Person Camera`))))
  ; Line Trace
  (bind (_outhit _returnvalue) (`KismetSystemLibrary.LineTraceSingle` :`Start` _returnvalue_location :`End` (+ _returnvalue_location (* (`KismetMathLibrary.GetForwardVector` (`self.RandomRotator` _returnvalue_rotation (* -1.0 _rangeinrandom) _rangeinrandom)) 4000)) :`TraceChannel` "TraceTypeQuery1" :`bIgnoreSelf` false))
  ; Spawn Actor in hit
  (if _returnvalue
    (bind (_bblockinghit _binitialoverlap _time _distance _location _impactpoint _normal _impactnormal _physmat _hitactor) (`GameplayStatics.BreakHitResult` _outhit))
    (bind _output_get (set `self.Phys Mat` _physmat))
    (if (not (== _output_get "/Game/Project/MaterialLibrary/Materials/PM_NotRecetiveToLidar.PM_NotRecetiveToLidar"))
      (set `self.Hit Actor` _hitactor)
      (bind _returnvalue_2 (`|SpawnActorFromClass` "/Game/Project/Blueprints/Actors/BP_Pixel.BP_Pixel_C" (`KismetMathLibrary.MakeTransform` _location) "Undefined" "MultiplyWithRoot" null (`self.As BP First Person Character`) null))
      (bind _output_get_2 (set `self.SpawnActor` _returnvalue_2))
      (`Actor.SetActorEnableCollision` _output_get_2 false)
      ; Set material (заготовка)
      (if (== (`self.Hit Actor`) "/Game/Project/Blueprints/BP_NPC.BP_NPC")
        (`/Game/Project/Blueprints/Actors/BP_Pixel.SetColorOnRed` (`self.SpawnActor`))))))

(event `Key|MouseScrollDown`
  (params (Key :type "Key Structure"))
  ; Range in Random
  (:`Pressed`
    (if (> (`self.RangeInRandom`) 1.0)
      (set `self.RangeInRandom` (- (`self.RangeInRandom`) 0.5)))))

(event `Key|MouseScrollUp`
  (params (Key :type "Key Structure"))
  ; Range in Random
  (:`Pressed`
    (if (< (`self.RangeInRandom`) 20.0)
      (set `self.RangeInRandom` (+ (`self.RangeInRandom`) 0.5)))))

(fn `isIgnorringActor`
  (return))

(fn `RandomRotator`
  (params (InRotator :type "Rotator Structure") (MinRandom :type "Float (double-precision)") (MaxRandom :type "Float (double-precision)"))
  (returns (OutRotator :type "Rotator Structure"))
  (return (`KismetMathLibrary.MakeRotator` (+ (.roll InRotator) (`KismetMathLibrary.RandomFloatInRange` MinRandom MaxRandom)) (+ (.pitch InRotator) (`KismetMathLibrary.RandomFloatInRange` MinRandom MaxRandom)) (+ (.yaw InRotator) (`KismetMathLibrary.RandomFloatInRange` MinRandom MaxRandom)))))